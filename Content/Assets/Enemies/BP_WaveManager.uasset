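; Wave manager actor that runs countdown-led enemy waves from a data table.
; On BeginPlay it sorts spawn points into Ground, Air, Tower and Special lists, then starts a looping one-second countdown timer.
; Each wave looks up the row named by its number and spawns enemies at random points of matching type, tracking them.
; A separate event, not called here, polls every second until all are invalid, then advances the wave and restarts the countdown.
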(event Custom|Countdown
  ;[1 1 1] Countdown
  (bind _returnvalue (Utilities|Time|SetTimerbyEvent (delegate Custom|Count) 1.0 true))
  (if (not (Variables|Default|GetIsInfCountdown))
    (Variables|Default|SetTime 3)))

(event Custom|Count
  ;[1 1 1] Countdown
  (Development|PrintString (Utilities|String|ToString(Integer) (Variables|Default|GetTime)))
  (Math|Integer|DecrementInt (Variables|Default|GetTime)
    (:%20%20
      (if (== (Variables|Default|GetTime) 0)
        (Utilities|Time|ClearandInvalidateTimerbyHandle (stale Custom|Countdown _returnvalue))
        (CallFunction|BeginWave)))))

(event Custom|BeginWave
  ;[1 1 1] Spawn Enemies for Wave
  (bind _returnvalue (Utilities|GetDataTableRow (Variables|Default|GetEnemyDataTable) (Utilities|String|StringToName (Utilities|String|ToString(Integer) (Variables|Default|GetWaveNumber))))
    (:then
      (for _array_element (Utilities|Struct|BreakWaveInfo _returnvalue)
        (CallFunction|SpawnEnemies)))
    (:RowNotFound
      (Development|PrintString "Couldn't find row for wave data"))))

(event Custom|StartCheckIfEnemiesAreDead
  ;[1 1 1] Check if enemies are dead and start new wave if they are
  (bind _aredead_ (CallFunction|CheckifAllEnemiesAreDead :!label _label))
  (if _aredead_
    (Audio|PlaySound2D "/Game/StarterContent/Audio/Collapse01.Collapse01" 1.0 1.0 0.0 0 0) ; Change Sound Asset Later. This is placeholder!
    (Math|Integer|IncrementInt (Variables|Default|GetWaveNumber)
      (:%20%20
        (CallFunction|Countdown)))
    (else
      (Utilities|FlowControl|Delay 1.0)
      (goto _label))))

(event EventBeginPlay
  ;[1 1 1] Sort Enemy Spawner References
  (bind _outactors (Actor|GetAllActorsOfClass "/Game/Assets/Enemies/BP_SpawnPoint.BP_SpawnPoint_C"))
  (bind _output_get (Variables|Default|SetSpawnPoints _outactors))
  (for _array_element _output_get
    (switch Utilities|FlowControl|Switch|SwitchonEnemyTypes_E (Variables|/Game/Assets/Enemies/BP_SpawnPoint.BP_SpawnPoint_C|GetSpawnerType _array_element)
      (:NewEnumerator0
        (Utilities|Array|Add (Variables|Default|GetE_Ground) _array_element))
      (:NewEnumerator1
        (Utilities|Array|Add (Variables|Default|GetE_Air) _array_element))
      (:NewEnumerator2
        (Utilities|Array|Add (Variables|Default|GetE_Tower) _array_element))
      (:NewEnumerator3
        (Utilities|Array|Add (Variables|Default|GetE_Special) _array_element))))
  (CallFunction|Countdown))

(fn ConstructionScript)

(fn SpawnEnemies
  (params (EnemyInfo :type Enemy%20Info%20Structure))
  (bind _goblincontroller (Variables|Default|GetGoblinController))
  (LocalVariables|SetEnemyInfoRef EnemyInfo)
  (LocalVariables|SetCurrentSpawnPoint (Utilities|Select :Index (.EnemyType (Utilities|Struct|BreakEnemyInfo EnemyInfo)) :NewEnumerator0 (Variables|Default|GetE_Ground) :NewEnumerator1 (Variables|Default|GetE_Air) :NewEnumerator2 (Variables|Default|GetE_Tower) :NewEnumerator3 (Variables|Default|GetE_Special)))
  (for _index (range 1 (.enemynum (LocalVariables|GetEnemyInfoRef)))
    (bind _returnvalue (Game|SpawnActorfromClass (.enemyclass (LocalVariables|GetEnemyInfoRef)) (Transformation|GetWorldTransform (Variables|/Game/Assets/Enemies/BP_SpawnPoint.BP_SpawnPoint_C|GetBillboard (Utilities|Array|Get(acopy) (LocalVariables|GetCurrentSpawnPoint) (Math|Random|RandomIntegerinRange 0 (Utilities|Array|LastIndex (LocalVariables|GetCurrentSpawnPoint)))))) "AlwaysSpawn" 0 0))
    (Utilities|Array|Add (Variables|Default|GetCurrentEnemies) _returnvalue)
    (Utilities|Casting|CastToAI_GoblinController _goblincontroller)
    (Variables|/Game/Assets/Enemies/AI_GoblinController.AI_GoblinController_C|SetCurrent%20Health _goblincontroller 1e+02)))

(fn CheckifAllEnemiesAreDead
  (Variables|Default|SetAreDead? true)
  (for _array_element (Variables|Default|GetCurrentEnemies)
    (Utilities|IsValid _array_element
      (:Is%20Valid
        (Variables|Default|SetAreDead? false))))
  (return (Variables|Default|GetAreDead?)))