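; Server-driven wave spawner that runs a start countdown, then spawns successive enemy waves until the final one is finished.
; Init loads wave settings from a data table row, collects WaveBasedSpawnPoint actors and seeds a random stream.
; Each wave spawns its enemy classes at seeded random points and yaws, filtered by spawn point index.
; It polls every second until all spawned references are invalid, with printed messages and sounds marking progress.
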(event Custom|SR_Display%20Message
  (params (InString :type String))
  ;[1 1 1] Display message
  (Development|PrintString InString true true "(R=0.000000,G=0.660000,B=1.000000,A=1.000000)" 1e+01))

(event Custom|SR_Spawn%20Next%20Wave
  ;[1 1 1] Spawn next wave
  ;;[1 1 1] Increment wave, start wave message and SFX
  (Math|Integer|IncrementInt (Variables|Default|GetcurrentWaveNumber)
    (:%20%20
      (CallFunction|SRDisplayMessage (Utilities|String|Append "Wave " (Utilities|String|ToString(Integer) (Variables|Default|GetcurrentWaveNumber)) " begin!"))
      (CallFunction|MCSpawnSound (Variables|SFX|GetSFX_StartWave))
      ;;[1 1 1] Spawn enemies, and check validity periodically
      (CallFunction|SpawnEnemiesforCurrentWave)
      (bind _alldefeated_ (CallFunction|CheckifEnemiesAreDefeated :!label _label))
      (if _alldefeated_
        ;;[1 1 1] Wave finished feedback
        (CallFunction|MCSpawnSound (Variables|SFX|GetSFX_FinishedWave))
        (CallFunction|SRDisplayMessage (Utilities|String|Append "Wave " (Utilities|String|ToString(Integer) (Variables|Default|GetcurrentWaveNumber)) " complete!"))
        (Utilities|FlowControl|Delay (Variables|Public|GetwaitBetweenWaves))
        ;;[1 1 1] Check if final wave?
        (if (== (Utilities|Array|LastIndex (Utilities|Struct|BreakwaveInfo_S (Variables|Default|GetwaveSettings))) (Variables|Default|GetcurrentWaveNumber))
          ;[1 1 1] Finish game, or start next wave
          (CallFunction|SRFinalWaveFinished)
          (else
            (CallFunction|SRSpawnNextWave)))
        (else
          (Utilities|FlowControl|Delay 1.0)
          (goto _label))))))

(event Custom|MC_SpawnSound
  (params (Sound :type Sound%20Base%20Object%20Reference))
  ;[1 1 1] MC_Spawn Sound
  (Audio|SpawnSound2D Sound 1.0 1.0 0.0 0))

(event Custom|SR_Final%20Wave%20Finished
  ;[1 1 1] Finished final wave
  (CallFunction|SRDisplayMessage "Final wave complete!")
  (CallFunction|MCSpawnSound (Variables|SFX|GetSFX_FinishedFinalWave)))

(event EventBeginPlay
  ;[1 1 1] BP: Server only
  (Networking|SwitchHasAuthority
    (:Authority
      (CallFunction|Init)
      ;;[1 1 1] Countdown until start
      (CallFunction|SRDisplayMessage (Utilities|String|Append "Time until start: " (Utilities|String|ToString(Integer) (Variables|Default|Getcounter))) :!label _label)
      (if (== (Variables|Default|Getcounter) 0)
        (CallFunction|SRSpawnNextWave)
        (else
          (Utilities|FlowControl|Delay 1.0)
          (Math|Integer|DecrementInt (Variables|Default|Getcounter)
            (:%20%20
              (goto _label))))))))

(fn ConstructionScript)

(fn Init
  ;[1 1 1] Data table
  (bind _returnvalue (Utilities|GetDataTableRow "/Game/WaveBasedSpawner/Blueprints/waveInfo_DT.waveInfo_DT" (Variables|Public|GetwaveSettingsRowName))
    (:then
      (Variables|Default|SetwaveSettings _returnvalue)
      ;[1 1 1] Counter
      (Variables|Default|Setcounter (Variables|Public|GetinitialCountdown))
      ;[1 1 1] Save spawn points
      (bind _outactors (Actor|GetAllActorsOfClass "/Game/WaveBasedSpawner/Blueprints/waveBasedSpawnPoint_BP.waveBasedSpawnPoint_BP_C"))
      (Variables|Default|SetspawnPointReferences _outactors)
      ;[1 1 1] Set seed
      (Math|Random|SetRandomStreamSeed (Variables|Default|GetrandomStream) (Variables|Public|Getseed)))))

(fn SpawnEnemiesforCurrentWave
  (bind _wavesettings (Variables|Default|GetwaveSettings))
  (bind _currentwavenumber (Variables|Default|GetcurrentWaveNumber))
  (bind _waveinfo (Utilities|Struct|BreakwaveInfo_S _wavesettings))
  (bind _output (Utilities|Array|Get(acopy) _waveinfo _currentwavenumber))
  (bind (_enemyclasses _classamount _spawnpointindex) (Utilities|Struct|BreakwaveEnemyInfo_S _output))
  (for (_array_element _array_index) _enemyclasses
    (for _index (range 1 (Utilities|Array|Get(acopy) _classamount _array_index))
      (bind _returnvalue (Game|SpawnActorfromClass _array_element (CallFunction|GetRandomSpawnPoint (Utilities|Array|Get(acopy) _spawnpointindex _array_index)) "Undefined" 0 0))
      (Utilities|Array|Add (Variables|Default|GetcurrentEnemyReferences) _returnvalue)))
  (return))

(fn GetRandomSpawnPoint
  (params (spawnPointIndex :type Integer))
  (return (Math|Transform|MakeTransform (Transformation|GetWorldLocation (Variables|/Game/WaveBasedSpawner/Blueprints/waveBasedSpawnPoint_BP.waveBasedSpawnPoint_BP_C|GetspawnPointTransformBillboard (.OutItem (Utilities|Array|RandomFromStream (CallFunction|GetSpawnPointsOfIndex spawnPointIndex) (Variables|Default|GetrandomStream))))) (Math|Rotator|MakeRotator 0.0 0.0 (Math|Random|RandomFloatinRangefromStream 0.0 3.6e+02 (Variables|Default|GetrandomStream))))))

(fn CheckifEnemiesAreDefeated
  (for _array_element (Variables|Default|GetcurrentEnemyReferences)
    (Utilities|IsValid _array_element
      (:Is%20Valid
        (return false))))
  (return true))

(fn GetSpawnPointsOfIndex
  (params (index :type Integer))
  (Utilities|Array|Clear (LocalVariables|GetspawnPoints))
  (for _array_element (Variables|Default|GetspawnPointReferences)
    (if (== (Variables|/Game/WaveBasedSpawner/Blueprints/waveBasedSpawnPoint_BP.waveBasedSpawnPoint_BP_C|GetspawnPointIndex _array_element) index)
      (Utilities|Array|Add (LocalVariables|GetspawnPoints) _array_element)))
  (return (LocalVariables|GetspawnPoints)))